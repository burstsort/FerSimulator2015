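; Interactive door (Vrata) that toggles open or closed on Interact unless it is locked or mid-swing.
; Tick advances a 0–1 state that drives the yaw swing and a sine dip of two handle parts early in the range, triggering playback near the closed end.
; The construction script selects glass, dark and handle variants, stores the initial yaw and mirrors handedness through negative actor scale, which also flips the rotation direction.
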(event OnComponentBeginOverlap(Box)
  (params (OtherActor :type Actor%20Object%20Reference) (OtherComp :type Primitive%20Component%20Object%20Reference) (OtherBodyIndex :type Integer) (bFromSweep :type Boolean) (SweepResult :type Hit%20Result%20Structure%20%28by%20ref%29)))

(event OnComponentEndOverlap(Box)
  (params (OtherActor :type Actor%20Object%20Reference) (OtherComp :type Primitive%20Component%20Object%20Reference) (OtherBodyIndex :type Integer)))

(event EventInteract
  (bind _stanje (Variables|Default|GetStanje))
  (if (and (not (Variables|Default|GetZakljucano)) (or (<= _stanje 0.0) (>= _stanje 1.0)))
    (Variables|Default|SetOtvorena (not (Variables|Default|GetOtvorena)))))

(event EventActorBeginOverlap
  (params (OtherActor :type Actor%20Object%20Reference)))

(event EventTick
  (params (DeltaSeconds :type Float%20%28single-precision%29))
  (bind _brzinaotvaranja (Variables|Default|GetBrzinaOtvaranja))
  (bind _returnvalue (* DeltaSeconds _brzinaotvaranja))
  (if (and (> (Variables|Default|GetStanje) 0.0) (not (Variables|Default|GetOtvorena)))
    (Variables|Default|SetStanje (+ (Variables|Default|GetStanje) (* -1.0 _returnvalue)))
    (Transformation|SetRelativeRotation (Class|KismetMathLibrary|MakeRot 0.0 (+ (Math|Float|Lerp 0.0 (* (Variables|Default|GetMaxKut) (.X (Math|Vector|BreakVector (Transformation|GetActorScale3D)))) (Math|Float|Clamp(Float) (Variables|Default|GetStanje))) (Variables|Default|GetPocetnaRot)) 0.0) false :!label _label)
    (Transformation|SetRelativeRotation (Class|KismetMathLibrary|MakeRot (* (Math|Float|Lerp 0.0 -45.0 (Math|Trig|Sin(Radians) (* (Math|Float|Clamp(Float) (Variables|Default|GetStanje) 0.0 0.25) (Math|Trig|GetPI) 4.0))) (.X (Math|Vector|BreakVector (Transformation|GetActorScale3D)))) 1.8e+02 1.8e+02) false)
    (Transformation|SetRelativeRotation (Class|KismetMathLibrary|MakeRot (* (Math|Float|Lerp 0.0 -45.0 (Math|Trig|Sin(Radians) (* (Math|Float|Clamp(Float) (Variables|Default|GetStanje) 0.0 0.25) (Math|Trig|GetPI) 4.0))) (.X (Math|Vector|BreakVector (Transformation|GetActorScale3D)))) 1.8e+02 0.0) false)
    (if (Math|Float|InRange(Float) (Variables|Default|GetStanje) 0.0 0.1)
      (if (Variables|Default|GetOtvorena)
        (bind _returnvalue_2 (Audio|Components|Audio|IsPlaying))
        (if (not _returnvalue_2)
          (Audio|Components|Audio|Play 0.0))
        (else
          (bind _returnvalue_3 (Audio|Components|Audio|IsPlaying))
          (if (not _returnvalue_3)
            (Audio|Components|Audio|Play 0.0)))))
    (elif (and (< (Variables|Default|GetStanje) 1.0) (Variables|Default|GetOtvorena))
      (Variables|Default|SetStanje (+ (Variables|Default|GetStanje) _returnvalue))
      (goto _label))))

(fn ConstructionScript
  (bind _tamna (Variables|Default|GetTamna))
  (bind _kvaka (Variables|Default|GetKvaka))
  (bind _staklo (Variables|Default|GetStaklo))
  (bind _returnvalue (not _staklo))
  (Rendering|SetVisibility _staklo false)
  (Rendering|SetVisibility _staklo false)
  (Rendering|SetVisibility _returnvalue false)
  (Rendering|SetVisibility _returnvalue false)
  (Rendering|SetVisibility _tamna false)
  (Rendering|SetVisibility (not _tamna) false)
  (Rendering|SetVisibility _kvaka false)
  (Rendering|SetVisibility _kvaka false)
  (Rendering|SetVisibility false true)
  (Variables|Default|SetPocetnaRot (.Yaw (Class|KismetMathLibrary|BreakRot (Transformation|GetActorRotation))))
  (Transformation|SetActorScale3D (Math|Vector|MakeVector (Math|Float|SelectFloat -1.0 1.0 (Variables|Default|GetDesna)) (Math|Float|SelectFloat -1.0 1.0 (Variables|Default|GetFlip)) 1.0)))