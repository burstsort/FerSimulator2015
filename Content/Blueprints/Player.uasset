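; Player pawn Blueprint that handles first-person-style movement, looking, interaction and quitting.
; Axis inputs move it along the control rotation's forward and right vectors and drive controller pitch and yaw.
; Interact fires a short Visibility line trace from above the actor's location along the view direction and calls InteractMessage on the hit actor.
; Escape quits the game.
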(event EventBeginPlay)

(event EventActorBeginOverlap
  (params (OtherActor :type Actor%20Object%20Reference)))

(event EventTick
  (params (DeltaSeconds :type Float%20%28single-precision%29)))

(event Input|ActionEvents|InputActionInteract
  (bind _returnvalue (Transformation|GetActorLocation))
  (bind _returnvalue_2 (+ _returnvalue "0, 0,100.000000"))
  (:Pressed
    (bind (_outhit _returnvalue_3) (Collision|LineTraceByChannel _returnvalue_2 (+ _returnvalue_2 (* (Math|Vector|GetForwardVector (Pawn|GetControlRotation :!class /Script/Engine.Pawn)) 2.5e+02)) "TraceTypeQuery1" false 0 "None"))
    (if _returnvalue_3
      (Class|Interactable|Interact(Message) (.HitActor (Collision|BreakHitResult _outhit))))))

(event Input|AxisEvents|InputAxisCameraForward
  (params (AxisValue :type Float%20%28single-precision%29))
  (Pawn|Input|AddMovementInput (Math|Vector|GetForwardVector (Pawn|GetControlRotation :!class /Script/Engine.Pawn)) AxisValue false))

(event Input|AxisEvents|InputAxisCameraRight
  (params (AxisValue :type Float%20%28single-precision%29))
  (Pawn|Input|AddMovementInput (Math|Vector|GetRightVector (Pawn|GetControlRotation :!class /Script/Engine.Pawn)) AxisValue false))

(event Input|AxisEvents|InputAxisCameraPitch
  (params (AxisValue :type Float%20%28single-precision%29))
  (Pawn|Input|AddControllerPitchInput AxisValue))

(event Input|AxisEvents|InputAxisCameraYaw
  (params (AxisValue :type Float%20%28single-precision%29))
  (Pawn|Input|AddControllerYawInput AxisValue))

(event Input|KeyboardEvents|Escape
  (:Pressed
    (Game|QuitGame 0 "Quit")))

(fn ConstructionScript)